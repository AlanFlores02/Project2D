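; Player-controlled Paper2D knight that runs along X, jumps, attacks, collects coins and takes damage.
; Capsule overlaps destroy non-imaginary coins and update the HUD created at BeginPlay, or apply damage from "Danger" actors, opening GameOverMap when health runs out.
; E triggers a grounded attack state that briefly slows walking, with no hit detection here.
; Each tick, PickAnim layers velocity and attack checks to choose the flipbook, facing and sprite offset.
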(event `self.ReceiveTick`
  (params (DeltaSeconds :type "Float (single-precision)"))
  (`self.PickAnim`))

(event `InputAxis|MoveRight`
  (params (AxisValue :type "Float (single-precision)"))
  ;[1 1 1] Inputs
  (`self.AddMovementInput` (1.0 0.0 0.0) AxisValue))

(event `InputAction|Jump`
  (params (Key :type "Key Structure"))
  ;[1 1 1] Inputs
  (:`Pressed`
    (`self.Jump`))
  (:`Released`
    (`self.StopJumping`)))

(event `self.CapsuleComponent.OnComponentBeginOverlap`
  (params (OverlappedComponent :type "PrimitiveComponent Object Reference") (OtherActor :type "Actor Object Reference") (OtherComp :type "PrimitiveComponent Object Reference") (OtherBodyIndex :type Integer) (bFromSweep :type Boolean) (SweepResult :type "HitResult Structure (by ref)"))
  ;[1 1 1] Collision
  (bind _asbp_coin (cast `/Game/Items/Coins/BP_Coin` OtherActor)
    (:`then`
      (if (not (`/Game/Items/Coins/BP_Coin.Imaginary` _asbp_coin))
        (`self.K2_DestroyActor` _asbp_coin)
        (`/Game/UI/Main_HUD.GainCoin` (`self.HUD`))))
    (:`CastFailed`
      (if (`self.ActorHasTag` OtherActor "Danger")
        (`GameplayStatics.ApplyDamage` self 1.0)))))

(event `self.ReceiveAnyDamage`
  (params (Damage :type "Float (single-precision)") (DamageType :type "DamageType Object Reference") (InstigatedBy :type "Controller Object Reference") (DamageCauser :type "Actor Object Reference"))
  (bind _output_get (set `self.Health` (- (`self.Health`) Damage)))
  (if (<= _output_get 0.0)
    (`GameplayStatics.OpenLevel` "GameOverMap")))

(event `Key|E`
  (params (Key :type "Key Structure"))
  (bind _charactermovement (`self.CharacterMovement`))
  (:`Pressed`
    (if (and (`NavMovementComponent.IsMovingOnGround` (`self.CharacterMovement`)) (not (`self.Attack`)))
      (set `CharacterMovementComponent.MaxWalkSpeed` 1.0 _charactermovement)
      (set `self.Attack` true)
      (`KismetSystemLibrary.RetriggerableDelay` 0.5)
      (set `CharacterMovementComponent.MaxWalkSpeed` 150.0 _charactermovement)
      (set `self.Attack` false))))

(fn `PickAnim`
  (locals (`Offset X` :type "Float (double-precision)" :default -15.0) (`Offset Z` :type "Float (double-precision)" :default -2.0))
  (bind _sprite (`self.Sprite`))
  (bind _direction (`self.Direction`))
  (bind (_velocity_x _velocity_y _velocity_z) (`KismetMathLibrary.BreakVector` (`MovementComponent.Velocity` (`self.CharacterMovement`))))
  (`|ExecutionSequence`
    (:`then_0`
      (`/Engine/EditorBlueprintResources/StandardMacros.CompareFloat` _velocity_x
        (:`>`
          (set `self.Direction` 1.0)
          (set `self.Animation` "/Game/Enemy/KnightPlayer/FB_RunKnight.FB_RunKnight" :!label _label))
        (:`==`
          (set `self.Animation` "/Game/Enemy/KnightPlayer/FB_IdleKnight.FB_IdleKnight"))
        (:`<`
          (set `self.Direction` -1.0)
          (goto _label))))
    (:`then_1`
      (`/Engine/EditorBlueprintResources/StandardMacros.CompareFloat` _velocity_z ; Falling or jumping
        (:`>`
          (set `self.Animation` "/Game/Enemy/KnightPlayer/FB_JumpKnight.FB_JumpKnight"))
        (:`<`
          (set `self.Animation` "/Game/Enemy/KnightPlayer/FB_FallKnight.FB_FallKnight"))))
    (:`then_2`
      (if (`self.Attack`)
        (set `self.Animation` "/Game/Enemy/KnightPlayer/FB_AttackKnight.FB_AttackKnight")
        (set `local.Offset X` 10.0)
        (set `local.Offset Z` 10.0)))
    (:`then_3`
      (`PaperFlipbookComponent.SetFlipbook` (`self.Sprite`) (`self.Animation`))
      (`SceneComponent.SetRelativeScale3D` _sprite (`KismetMathLibrary.MakeVector` _direction 1.0 1.0))
      (`SceneComponent.K2_SetRelativeLocation` _sprite (`KismetMathLibrary.MakeVector` (* _direction (`local.Offset X`)) 0.0 (`local.Offset Z`)) false false))))

(fn `ReceiveBeginPlay`
  (bind _returnvalue (`|CreateWidget` "/Game/UI/Main_HUD.Main_HUD_C"))
  (bind _output_get (set `self.HUD` _returnvalue))
  (`UserWidget.AddToViewport` _output_get 0))

(fn `UserConstructionScript`)