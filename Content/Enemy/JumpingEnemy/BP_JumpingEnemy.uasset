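; Paper2D frog enemy character that hops horizontally on a looping timer.
; Each timer tick saves its location, jumps and adds an X velocity impulse along Direction.
; On landing, if it has barely moved from the saved spot, it reverses Direction and mirrors the sprite to match.
; Tick picks the jump, idle or fall flipbook from the sign of vertical velocity.
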(event `self.ReceiveTick`
  (params (DeltaSeconds :type "Float (single-precision)"))
  (`self.Pick Anim`))

(event `self.ReceiveBeginPlay`
  (`KismetSystemLibrary.K2_SetTimerDelegate` (delegate `Jump Timer`) 3.0 true))

(event `Jump Timer`
  (if (`self.CanJump`)
    (set `self.LastPos` (`self.K2_GetActorLocation`))
    (`self.Jump`)
    (`CharacterMovementComponent.AddImpulse` (`self.CharacterMovement`) (`KismetMathLibrary.MakeVector` (* 200.0 (`self.Direction`))) true)))

(event `self.OnLanded`
  (params (Hit :type "HitResult Structure (by ref)"))
  (bind _direction (`self.Direction`))
  (if (< (`KismetMathLibrary.Vector_Distance` (`self.K2_GetActorLocation`) (`self.LastPos`)) 20.0)
    (`/Engine/EditorBlueprintResources/StandardMacros.NegateFloat` _direction
      (:`  `
        (`SceneComponent.SetRelativeScale3D` (`self.Sprite`) (`KismetMathLibrary.MakeVector` _direction 1.0 1.0))))))

(fn `Pick Anim`
  (bind _sprite (`self.Sprite`))
  (bind (_velocity_x _velocity_y _velocity_z) (`KismetMathLibrary.BreakVector` (`MovementComponent.Velocity` (`self.CharacterMovement`))))
  (`/Engine/EditorBlueprintResources/StandardMacros.CompareFloat` _velocity_z
    (:`>`
      (`PaperFlipbookComponent.SetFlipbook` _sprite "/Game/Enemy/JumpingEnemy/Sprites/FB_PhrogJump.FB_PhrogJump"))
    (:`==`
      (`PaperFlipbookComponent.SetFlipbook` _sprite "/Game/Enemy/JumpingEnemy/Sprites/FB_PhrogIdle.FB_PhrogIdle"))
    (:`<`
      (`PaperFlipbookComponent.SetFlipbook` _sprite "/Game/Enemy/JumpingEnemy/Sprites/FB_PhrogFall.FB_PhrogFall"))))

(fn `UserConstructionScript`)