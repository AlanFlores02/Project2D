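; Goblin side-scrolling character that autonomously collects BP_Coin actors in AIPathOrder, opening GameOverMap when damage depletes its health.
; BeginPlay sorts the coins with a swap sort; each capsule overlap with a coin destroys it and advances the goal index.
; Tick steers along X toward the current coin, jumping for raised coins or based on box traces for holes and obstacles.
; PickAnim sets flipbook and sprite facing from velocity.
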(event `self.ReceiveTick`
  (params (DeltaSeconds :type "Float (single-precision)"))
  (`self.PickAnim`)
  (`self.AI Movement`))

(event `self.ReceiveBeginPlay`
  (bind _outactors (`GameplayStatics.GetAllActorsOfClass` "/Game/Items/Coins/BP_Coin.BP_Coin_C"))
  (bind _sorted_array (`self.Sort Actor Array` _outactors))
  (set `self.Goal Array` _sorted_array))

(event `self.ReceiveAnyDamage`
  (params (Damage :type "Float (single-precision)") (DamageType :type "DamageType Object Reference") (InstigatedBy :type "Controller Object Reference") (DamageCauser :type "Actor Object Reference"))
  ;[1 1 1] Die
  (bind _output_get (set `self.Health` (- (`self.Health`) Damage)))
  (if (<= _output_get 0.0)
    (`GameplayStatics.OpenLevel` "GameOverMap")))

(event `self.CapsuleComponent.OnComponentBeginOverlap`
  (params (OverlappedComponent :type "PrimitiveComponent Object Reference") (OtherActor :type "Actor Object Reference") (OtherComp :type "PrimitiveComponent Object Reference") (OtherBodyIndex :type Integer) (bFromSweep :type Boolean) (SweepResult :type "HitResult Structure (by ref)"))
  ;[1 1 1] Collision
  (bind _asbp_coin (cast `/Game/Items/Coins/BP_Coin` OtherActor))
  (`/Engine/EditorBlueprintResources/StandardMacros.IncrementInt` (`self.Current Goal`)
    (:`  `
      (`self.K2_DestroyActor` _asbp_coin))))

(event `AI Movement`
  (bind (_returnvalue_x _returnvalue_y _returnvalue_z) (`KismetMathLibrary.BreakVector` (`self.K2_GetActorLocation`)))
  (bind _goal_array (`self.Goal Array`))
  (bind _current_goal (`self.Current Goal`))
  (bind (_returnvalue_x_2 _returnvalue_y_2 _returnvalue_z_2) (`KismetMathLibrary.BreakVector` (`self.K2_GetActorLocation` (`|GetArrayItem` _goal_array _current_goal))))
  (bind _returnvalue (- _returnvalue_z_2 _returnvalue_z))
  (bind _returnvalue_2 (- _returnvalue_x_2 _returnvalue_x))
  ;[1 1 1] Simple Movement: walk to the next coin
  (if (> (`KismetArrayLibrary.Array_Length` _goal_array) _current_goal)
    (`|ExecutionSequence`
      (:`then_0`
        (`self.AddMovementInput` (`KismetMathLibrary.MakeVector` (`KismetMathLibrary.FClamp` _returnvalue_2 -1.0))))
      (:`then_1`
        (if (and (< (`KismetMathLibrary.Abs` _returnvalue_2) 30.0) (> _returnvalue 20.0) (< _returnvalue 60.0))
          (`self.Jump` :!label _label)
          (else
            (`self.AI Jump Over Holes`)
            (`self.AI Jump Over Obstacle`)))))))

(event `AI Jump Over Holes`
  (bind _returnvalue (+ (`self.K2_GetActorLocation`) (`KismetMathLibrary.MakeVector` (* (`self.Direction`) 10.0))))
  (bind (_outhit _returnvalue_2) (`KismetSystemLibrary.BoxTraceSingle` :`Start` _returnvalue :`End` (- _returnvalue (0.0 0.0 20.0)) :`HalfSize` (5.0 5.0 5.0) :`TraceChannel` "TraceTypeQuery1" :`DrawDebugType` "ForOneFrame" :`TraceColor` (struct :`R` 0.8 :`G` 0.2 :`A` 1.0) :`TraceHitColor` (struct :`R` 0.2 :`A` 1.0)))
  (if (not _returnvalue_2)
    (goto _label)))

(event `AI Jump Over Obstacle`
  (bind _returnvalue (* (`self.Direction`) 10.0))
  (bind _returnvalue_2 (+ (`self.K2_GetActorLocation`) (`KismetMathLibrary.MakeVector` _returnvalue 0.0 -5.0)))
  (bind (_outhit _returnvalue_3) (`KismetSystemLibrary.BoxTraceSingle` :`Start` _returnvalue_2 :`End` (+ _returnvalue_2 (`KismetMathLibrary.MakeVector` _returnvalue 0.0 10.0)) :`TraceChannel` "TraceTypeQuery1" :`DrawDebugType` "ForOneFrame" :`TraceColor` (struct :`R` 0.2 :`G` 0.2 :`B` 1.0 :`A` 1.0) :`TraceHitColor` (struct :`B` 0.8 :`A` 1.0)))
  (if (not _returnvalue_3)
    (`KismetSystemLibrary.RetriggerableDelay` 0.5)
    (goto _label)))

(fn `Actor Sort Function`
  (params (`Actor 1` :type "/Game/Items/Coins/BP_Coin Object Reference") (`Actor 2` :type "/Game/Items/Coins/BP_Coin Object Reference"))
  (returns (`A is bigger` :type Boolean))
  (return (< (`/Game/Items/Coins/BP_Coin.AI Path Order` `Actor 1`) (`/Game/Items/Coins/BP_Coin.AI Path Order` `Actor 2`))))

(fn `PickAnim`
  (bind _not_broken (`self.Not Broken`))
  (bind (_velocity_x _velocity_y _velocity_z) (`KismetMathLibrary.BreakVector` (`MovementComponent.Velocity` (`self.CharacterMovement`))))
  (set `self.Not Broken` true)
  (`|ExecutionSequence`
    (:`then_0`
      (`/Engine/EditorBlueprintResources/StandardMacros.CompareFloat` _velocity_z ; Falling or jumping
        (:`>`
          (set `self.Animation` "/Game/Enemy/GoblinEnemy/FB_Goblin_Jump.FB_Goblin_Jump"))
        (:`<`
          (set `self.Animation` "/Game/Enemy/GoblinEnemy/FB_Goblin_Fall.FB_Goblin_Fall")))
      (set `self.Not Broken` false))
    (:`then_1`
      (`/Engine/EditorBlueprintResources/StandardMacros.CompareFloat` _velocity_x
        (:`>`
          (set `self.Direction` 1.0)
          (`SceneComponent.SetRelativeScale3D` (`self.Sprite`) (`KismetMathLibrary.MakeVector` (`self.Direction`) 1.0 1.0) :!label _label)
          (if _not_broken
            (set `self.Animation` "/Game/Enemy/GoblinEnemy/FB_Goblin_Walk.FB_Goblin_Walk")))
        (:`==`
          (if _not_broken
            (set `self.Animation` "/Game/Enemy/GoblinEnemy/FB_Goblin_Idle.FB_Goblin_Idle")))
        (:`<`
          (set `self.Direction` -1.0)
          (goto _label))))
    (:`then_2`
      (`PaperFlipbookComponent.SetFlipbook` (`self.Sprite`) (`self.Animation`)))))

(fn `Sort Actor Array`
  (params (`Array to Sort` :type "Array of /Game/Items/Coins/BP_Coin Object Reference"))
  (returns (`Sorted Array` :type "Array of /Game/Items/Coins/BP_Coin Object Reference"))
  (locals (Sorted :type "Array of /Game/Items/Coins/BP_Coin Object Reference"))
  (bind _output_get (set `local.Sorted` `Array to Sort`))
  (bind _returnvalue (`KismetArrayLibrary.Array_Length` _output_get))
  (for _index (range (+ (- _returnvalue 2) 1))
    (for _index_2 (range (+ _index 1) _returnvalue)
      (bind _a_is_bigger (`self.Actor Sort Function` (`|GetArrayItem` _output_get _index_2) (`|GetArrayItem` _output_get _index)))
      (if _a_is_bigger
        (`KismetArrayLibrary.Array_Swap` _output_get _index _index_2))))
  (return _output_get))

(fn `UserConstructionScript`)