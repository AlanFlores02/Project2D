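; BP_EnemyCrawler is a side-view crawler enemy that walks continuously along the world X axis and turns at walls.
; Every Tick it adds forced movement input along Direction and runs a short forward Visibility trace that ignores BP_Player actors, with debug drawing on.
; A hit updates Direction and mirrors the sprite through its X scale.
; A timer-reset flag then pauses wall checks briefly to prevent rapid re-turning.
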(event `self.ReceiveTick`
  (params (DeltaSeconds :type "Float (single-precision)"))
  (`self.Movement`)
  (if (`self.DontSpamTurning`)
    (`self.DontWalkIntoWalls`)))

(fn `Allow Turning`
  (set `self.DontSpamTurning` true))

(fn `DontWalkIntoWalls`
  (bind _returnvalue (`self.K2_GetActorLocation`))
  (bind _direction (`self.Direction`))
  (bind _outactors (`GameplayStatics.GetAllActorsOfClass` "/Game/Player/BP_Player.BP_Player_C"))
  (bind (_outhit _returnvalue_2) (`KismetSystemLibrary.LineTraceSingle` _returnvalue (+ _returnvalue (`KismetMathLibrary.MakeVector` (* 50.0 (`self.Direction`)))) "TraceTypeQuery1" false _outactors "ForOneFrame"))
  (if _returnvalue_2
    (`/Engine/EditorBlueprintResources/StandardMacros.NegateFloat` _direction
      (:`  `
        (`SceneComponent.SetRelativeScale3D` (`self.Sprite`) (`KismetMathLibrary.MakeVector` _direction 1.0 1.0))
        (set `self.DontSpamTurning` false)
        (`KismetSystemLibrary.K2_SetTimer` null "Allow Turning" 1.0)))))

(fn `Movement`
  (`self.AddMovementInput` (1.0 0.0 0.0) (`self.Direction`) true))

(fn `UserConstructionScript`)