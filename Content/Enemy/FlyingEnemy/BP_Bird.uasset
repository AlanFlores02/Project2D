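; BP_Bird is a flying enemy that patrols horizontally and drops BP_Poopie projectiles on targets below.
; Tick moves it along X by MoveSpeed times its State direction and box-traces downward, leading by one speed unit.
; A hit on the target class triggers a drop with an impulse along the flight direction, gated by a reload delay.
; Collider overlaps update State and the mirrored X scale, apparently reversing direction.
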(event `self.ReceiveTick`
  (params (DeltaSeconds :type "Float (single-precision)"))
  (bind _returnvalue (`self.K2_GetActorLocation`))
  (`self.K2_AddActorWorldOffset` (`KismetMathLibrary.MakeVector` (* DeltaSeconds (* (`self.MoveSpeed`) (`self.State`)))) true)
  (bind _outhit (`KismetSystemLibrary.BoxTraceSingle` :`Start` _returnvalue :`End` (+ _returnvalue (`KismetMathLibrary.MakeVector` (* (`self.State`) (`self.MoveSpeed`)) 0.0 -400.0)) :`HalfSize` (5.0 5.0 5.0) :`TraceChannel` "TraceTypeQuery1" :`DrawDebugType` "ForOneFrame"))
  (cast `/Game/Enemy/FlyingEnemy/BP_` (`.HitActor` (`GameplayStatics.BreakHitResult` _outhit)))
  (if (`self.CaquitaReady`)
    (set `self.CaquitaReady` false)
    (`self.Cagar`)
    (`KismetSystemLibrary.Delay` (`self.ReloadTime`))
    (set `self.CaquitaReady` true)))

(event `self.Collider.OnComponentBeginOverlap`
  (params (OverlappedComponent :type "PrimitiveComponent Object Reference") (OtherActor :type "Actor Object Reference") (OtherComp :type "PrimitiveComponent Object Reference") (OtherBodyIndex :type Integer) (bFromSweep :type Boolean) (SweepResult :type "HitResult Structure (by ref)"))
  (bind _state (`self.State`))
  (`self.SetActorScale3D` (`KismetMathLibrary.MakeVector` _state 1.0 1.0))
  (`/Engine/EditorBlueprintResources/StandardMacros.NegateFloat` _state))

(event `Cagar`
  (bind _returnvalue (`|SpawnActorFromClass` "/Game/Enemy/FlyingEnemy/BP_Poopie.BP_Poopie_C" (`KismetMathLibrary.MakeTransform` (`self.K2_GetActorLocation`)) "AlwaysSpawn" "OverrideRootScale" null null))
  (`PrimitiveComponent.AddImpulse` (`PaperSpriteActor.RenderComponent` _returnvalue) (`KismetMathLibrary.MakeVector` (* (`self.State`) (`self.MoveSpeed`))) "None" false))

(fn `UserConstructionScript`)