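; Player character for a 2D side-scrolling platformer, with horizontal movement, jumping, coin pickup and health.
; Each Tick, PickAnim picks the flipbook from velocity, letting jump and fall override run and idle, and mirrors the sprite by X scale.
; Capsule overlaps collect coins into the Main_HUD widget or take damage from "Danger"-tagged actors, opening GameOverMap when health runs out.
; The older UpdateAnimation and UpdateControlRotation events are never called.
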(event `self.ReceiveTick`
  (params (DeltaSeconds :type "Float (single-precision)"))
  (`self.PickAnim`))

(event `InputAxis|MoveRight`
  (params (AxisValue :type "Float (single-precision)"))
  ;[1 1 1] Inputs
  (`self.AddMovementInput` (1.0 0.0 0.0) AxisValue))

(event `InputAction|Jump`
  (params (Key :type "Key Structure"))
  ;[1 1 1] Inputs
  (:`Pressed`
    (`self.Jump`))
  (:`Released`
    (`self.StopJumping`)))

(event `self.CapsuleComponent.OnComponentBeginOverlap`
  (params (OverlappedComponent :type "PrimitiveComponent Object Reference") (OtherActor :type "Actor Object Reference") (OtherComp :type "PrimitiveComponent Object Reference") (OtherBodyIndex :type Integer) (bFromSweep :type Boolean) (SweepResult :type "HitResult Structure (by ref)"))
  (bind _asbp_coin (cast `/Game/Items/Coins/BP_Coin` OtherActor)
    (:`then`
      (`self.K2_DestroyActor` _asbp_coin)
      (`/Game/UI/Main_HUD.GainCoin` (`self.HUD`)))
    (:`CastFailed`
      (if (`self.ActorHasTag` OtherActor "Danger")
        (`GameplayStatics.ApplyDamage` self 1.0)))))

(event `UpdateAnimation`
  ;[1 1 1] Old
  (`PaperFlipbookComponent.SetFlipbook` (`self.Sprite`) (select `bool` (`NavMovementComponent.IsFalling` (`self.CharacterMovement`)) :`false` (select `bool` (> (`KismetMathLibrary.VSize` (`MovementComponent.Velocity` (`self.CharacterMovement`))) 0.0) :`false` "/Game/Player/idle/FB_FoxIdle.FB_FoxIdle" :`true` "/Game/Player/run/FB_FoxRun.FB_FoxRun" :!type "PaperFlipbook Object Reference") :`true` "/Game/Player/fall/FB_Fall.FB_Fall")))

(event `UpdateControlRotation`
  ;[1 1 1] Old
  (`/Engine/EditorBlueprintResources/StandardMacros.IsValid` (`self.GetController`)
    (:`Is Valid`
      (`/Engine/EditorBlueprintResources/StandardMacros.CompareFloat` (.x (`MovementComponent.Velocity` (`self.CharacterMovement`)))
        (:`>`
          (`Controller.SetControlRotation` (`self.GetController`) (`KismetMathLibrary.MakeRotator` 0.0)))
        (:`<`
          (`Controller.SetControlRotation` (`self.GetController`) (`KismetMathLibrary.MakeRotator` 0.0 0.0 180.0)))))))

(event `self.ReceiveAnyDamage`
  (params (Damage :type "Float (single-precision)") (DamageType :type "DamageType Object Reference") (InstigatedBy :type "Controller Object Reference") (DamageCauser :type "Actor Object Reference"))
  (bind _output_get (set `self.Health` (- (`self.Health`) Damage)))
  (if (<= _output_get 0.0)
    (`GameplayStatics.OpenLevel` "GameOverMap")))

(fn `PickAnim`
  (bind _not_broken (`self.Not Broken`))
  (bind (_velocity_x _velocity_y _velocity_z) (`KismetMathLibrary.BreakVector` (`MovementComponent.Velocity` (`self.CharacterMovement`))))
  (set `self.Not Broken` true)
  (`|ExecutionSequence`
    (:`then_0`
      (`/Engine/EditorBlueprintResources/StandardMacros.CompareFloat` _velocity_z ; Falling or jumping
        (:`>`
          (set `self.Animation` "/Game/Player/jump/FB_Jump.FB_Jump"))
        (:`<`
          (set `self.Animation` "/Game/Player/fall/FB_Fall.FB_Fall")))
      (set `self.Not Broken` false))
    (:`then_1`
      (`/Engine/EditorBlueprintResources/StandardMacros.CompareFloat` _velocity_x
        (:`>`
          (set `self.Direction` 1.0)
          (`SceneComponent.SetRelativeScale3D` (`self.Sprite`) (`KismetMathLibrary.MakeVector` (`self.Direction`) 1.0 1.0) :!label _label)
          (if _not_broken
            (set `self.Animation` "/Game/Player/run/FB_FoxRun.FB_FoxRun")))
        (:`==`
          (if _not_broken
            (set `self.Animation` "/Game/Player/idle/FB_FoxIdle.FB_FoxIdle")))
        (:`<`
          (set `self.Direction` -1.0)
          (goto _label))))
    (:`then_2`
      (`PaperFlipbookComponent.SetFlipbook` (`self.Sprite`) (`self.Animation`)))))

(fn `ReceiveBeginPlay`
  (bind _returnvalue (`|CreateWidget` "/Game/UI/Main_HUD.Main_HUD_C"))
  (bind _output_get (set `self.HUD` _returnvalue))
  (`UserWidget.AddToViewport` _output_get 0))

(fn `UserConstructionScript`)